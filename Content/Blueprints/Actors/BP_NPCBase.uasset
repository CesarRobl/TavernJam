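; Base NPC actor that feeds dialogue lines to the player one at a time.
; On BeginPlay it copies the line text from every DT_DialogueInfo row into a Lines array.
; Each Talk event increments TalkIndex, then passes that line and a hardcoded speaker name to StartDialogue on BP_TopDownPlayerController.
; The index has no bounds check or reset.
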(event `self.ReceiveBeginPlay`
  (bind _lines (`self.Lines`))
  (bind _outrownames (`DataTableFunctionLibrary.GetDataTableRowNames` "/Game/Blueprints/Game_System/DT_DialogueInfo.DT_DialogueInfo"))
  (for _array_element _outrownames
    (bind _returnvalue (`|GetDataTableRow` "/Game/Blueprints/Game_System/DT_DialogueInfo.DT_DialogueInfo" _array_element)
      (:`then`
        (`KismetArrayLibrary.Array_Add` _lines (`.LineText` (break `DialogueData` _returnvalue)))
        (for _ _lines
          _)))))

(event `/Game/Blueprints/BPI_Dialogue.Talk`
  (`/Engine/EditorBlueprintResources/StandardMacros.IncrementInt` (`self.TalkIndex`)
    (:`  `
      (bind _asbp_top_down_player_controller (cast `/Game/Blueprints/Game_System/BP_TopDownPlayerController` (`GameplayStatics.GetPlayerController` 0)))
      (`/Game/Blueprints/Game_System/BP_TopDownPlayerController.StartDialogue` _asbp_top_down_player_controller "Gay" (`|GetArrayItem` (`self.Lines`) (`self.TalkIndex`))))))

(fn `UserConstructionScript`)