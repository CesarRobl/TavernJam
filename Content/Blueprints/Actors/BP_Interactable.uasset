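; Interactable actor that runs table-driven dialogue through BP_TopDownPlayerController.
; On BeginPlay it builds SDialogue from DT_Dialogue rows named by row prefix and index, as specified by DSet, which SetDialogue can change.
; Each Talk call registers it with the controller, then either skips to the finished line or starts the next one.
; After the last line it sends responses gathered from DT_Responses, or clears the dialogue if there are none.
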(event `self.ReceiveBeginPlay`
  (`self.GetDialogue`)
  (bind _asbp_top_down_player_controller (cast `/Game/Blueprints/Game_System/BP_TopDownPlayerController` (`GameplayStatics.GetPlayerController` 0)))
  (set `self.As BP Top Down Player Controller` _asbp_top_down_player_controller))

(event `/Game/Blueprints/BPI_Dialogue.Talk`
  (bind _as_bp_top_down_player_controller (`self.As BP Top Down Player Controller`))
  (bind (_s_dialogue_reponsetoget _s_dialogue_name _s_dialogue_lines _s_dialogue_responseamount) (break `/Game/Blueprints/Game_System/S_Dialogue` (`self.S Dialogue`)))
  (bind (_s_dialogue_reponsetoget_2 _s_dialogue_name_2 _s_dialogue_lines_2) (break `/Game/Blueprints/Game_System/S_Dialogue` (`self.S Dialogue`)))
  (set `/Game/Blueprints/Game_System/BP_TopDownPlayerController.Interactable` self _as_bp_top_down_player_controller)
  (bind _istalking (`/Game/Blueprints/Game_System/BP_TopDownPlayerController.IsDoneTalking` _as_bp_top_down_player_controller))
  (if _istalking
    (`/Engine/EditorBlueprintResources/StandardMacros.IncrementInt` (`self.TalkIndex`)
      (:`  `
        (if (>= (`self.TalkIndex`) (`KismetArrayLibrary.Array_Length` _s_dialogue_lines))
          (if (> _s_dialogue_responseamount 0)
            (set `self.TalkIndex` -1)
            (`self.GetResponses`)
            (`/Game/Blueprints/Game_System/BP_TopDownPlayerController.SendResponses` (`self.As BP Top Down Player Controller`) (`self.S Response`))
            (else
              (set `self.TalkIndex` -1)
              (`/Game/Blueprints/Game_System/BP_TopDownPlayerController.ClearDialogue` (`self.As BP Top Down Player Controller`) true)))
          (else
            (`/Game/Blueprints/Game_System/BP_TopDownPlayerController.StartDialogue` (`self.As BP Top Down Player Controller`) _s_dialogue_name_2 (`|GetArrayItem` _s_dialogue_lines_2 (`self.TalkIndex`)))))))
    (else
      (`/Game/Blueprints/Game_System/BP_TopDownPlayerController.SkipToFinishedLine` (`self.As BP Top Down Player Controller`)))))

(fn `ClearDialogue`
  (bind (_s_dialogue_reponsetoget _s_dialogue_name _s_dialogue_lines) (break `/Game/Blueprints/Game_System/S_Dialogue` (`self.S Dialogue`)))
  (`KismetArrayLibrary.Array_Clear` _s_dialogue_lines))

(fn `GetDialogue`
  (locals (NewLocalVar :type "Array of String"))
  (bind _newlocalvar (`local.NewLocalVar`))
  (bind (_d_set_rowname _d_set_lineamount) (break `/Game/Blueprints/Game_System/S_DialgoueSet` (`self.D Set`)))
  (for _index (range _d_set_lineamount)
    (bind _returnvalue (`|GetDataTableRow` "/Game/Blueprints/Game_System/DT_Dialogue.DT_Dialogue" (`KismetStringLibrary.Conv_StringToName` (`KismetStringLibrary.Concat_StrStr` (`KismetStringLibrary.Concat_StrStr` _d_set_rowname "_") (`KismetStringLibrary.Conv_IntToString` _index))))
      (:`then`
        (`KismetArrayLibrary.Array_Add` _newlocalvar (`.LineText` (break `DialogueData` _returnvalue)))
        (set `self.S Dialogue` (make `/Game/Blueprints/Game_System/S_Dialogue` (`.ResponseID` (break `DialogueData` _returnvalue)) (`.SpeakerName` (break `DialogueData` _returnvalue)) _newlocalvar (`.ResponseAmount` (break `DialogueData` _returnvalue))))))))

(fn `GetResponses`
  (locals (Index :type Integer))
  (bind (_s_dialogue_reponsetoget _s_dialogue_name _s_dialogue_lines _s_dialogue_responseamount) (break `/Game/Blueprints/Game_System/S_Dialogue` (`self.S Dialogue`)))
  (for _index (range _s_dialogue_responseamount)
    (bind _returnvalue (`|GetDataTableRow` "/Game/Blueprints/Game_System/DT_Responses.DT_Responses" (`KismetStringLibrary.Conv_StringToName` (`KismetStringLibrary.Concat_StrStr` (`KismetStringLibrary.Concat_StrStr` _s_dialogue_reponsetoget "_") (`KismetStringLibrary.Conv_IntToString` _index))))
      (:`then`
        (`self.SetResponseStruct` (break `ResponseData` _returnvalue) (`.ResponseID` (break `ResponseData` _returnvalue)) (`.LineAmount` (break `ResponseData` _returnvalue)) (`.ActionTag` (break `ResponseData` _returnvalue)))))))

(fn `SetDialogue`
  (params (NameToGet :type String) (Lines :type Integer))
  (returns (LineAmount :type Integer))
  (bind _output_get (set `self.D Set` (make `/Game/Blueprints/Game_System/S_DialgoueSet` NameToGet Lines)))
  (return (`.LineAmount_7_3EF0C0514838C67C048AF2B57911A26E` (break `/Game/Blueprints/Game_System/S_DialgoueSet` _output_get))))

(fn `SetResponseStruct`
  (params (Line :type String) (ID :type String) (LineAmount :type Integer) (Tag :type "GameplayTag Structure"))
  (bind (_s_response_responses _s_response_responseid_list _s_response_responseamount _s_response_tag) (break `/Game/Blueprints/Game_System/S_Response` (`self.S Response`)))
  (`|ExecutionSequence`
    (:`then_0`
      (`KismetArrayLibrary.Array_Add` _s_response_responses Line))
    (:`then_1`
      (`KismetArrayLibrary.Array_Add` _s_response_responseid_list ID))
    (:`then_2`
      (`KismetArrayLibrary.Array_Add` _s_response_responseamount LineAmount))
    (:`then_3`
      (`KismetArrayLibrary.Array_Add` _s_response_tag Tag))))

(fn `UserConstructionScript`)